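; Pistol weapon Blueprint for player character 0, with magazine ammo, a timed animated reload and a laser-dot sight.
; Tick sets bullet spray from crouch state and, when locally controlled, traces from the muzzle socket to redraw a short-lived laser decal.
; Firing repeats that trace, damaging BP_Guard hits, then spawns impact effects and a bullet actor, updates ammo and reports noise and damage events.
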(event EventBeginPlay
  (|CallParentFunction))

(event Collision|EventActorBeginOverlap
  (params (OtherActor :type Actor%20Object%20Reference))
  (|CallParentFunction OtherActor) ; This node is disabled and will not be called.\nDrag off pins to build functionality.
)

(event EventReloadWeapon
  ;[1 1 1] Reload
  (Components|Animation|PlayAnimation (Variables|Default|GetWeapon) "/Game/MilitaryWeapSilver/Weapons/Animations/Reload_Pistol_W.Reload_Pistol_W" false)
  (Utilities|FlowControl|Delay (Variables|Default|GetReloadTime))
  (Variables|Default|SetCurrentBullets (Variables|Default|GetMax_Bullets)))

(event EventFireWeapon
  ;[1 1 1] Shoot
  (if (> (Variables|Default|GetCurrentBullets) 0)
    (bind (_start_location _end_location _hit_actor) (CallFunction|LineTrace))
    (Class|Actor|MakeNoise 1.0 0 _end_location 0.0 "None")
    (CallFunction|SpawnDecalTracer _start_location _end_location _end_location)
    (Effects|SpawnEmitteratLocation "/Game/MilitaryWeapSilver/FX/P_Impact_Metal_Large_01.P_Impact_Metal_Large_01" _end_location)
    (CallFunction|AmmoCheck)
    (Class|AISenseDamage|ReportDamageEvent _hit_actor self (Variables|Default|GetDamage) (Transformation|GetActorLocation) "0, 0, 0" "None")
    (else
      (Audio|PlaySoundatLocation "/Game/Sounds/Weapons/Pistol/Fire_withoutBullet.Fire_withoutBullet" (Transformation|GetActorLocation) "0, 0, 0" 1.0 1.0 0.0 0 0 0 0))))

(event EventTick
  (params (DeltaSeconds :type Float%20%28single-precision%29))
  (|CallParentFunction DeltaSeconds)
  (if (Variables|/Script/Engine.Character|GetbIsCrouched (.AsPlayer%20Character (Utilities|Casting|CastToPlayer_character (Game|GetPlayerCharacter 0))))
    (Variables|Default|SetBullet%20spray 5e+01)
    (else
      (Variables|Default|SetBullet%20spray 75.0)))
  (if (Pawn|IsLocallyControlled (.AsPlayer%20Character (Utilities|Casting|CastToPlayer_character (Game|GetPlayerCharacter 0))))
    (CallFunction|LaserfromWeapon)))

(fn ConstructionScript
  (|CallParentFunction)
  (bind _output_get (Variables|Default|SetMax_Bullets 10))
  (Variables|Default|SetCurrentBullets _output_get)
  (Variables|Default|SetFireRate 0.5)
  (Variables|Default|SetReloadTime 2.0)
  (Variables|Default|SetBullet%20spray 75.0))

(fn AmmoCheck
  (if (not (Variables|/Game/ThirdPerson/Blueprints/Player_character.Player_character_C|GetIsReload (.AsPlayer%20Character (Utilities|Casting|CastToPlayer_character (Game|GetPlayerCharacter 0)))))
    (Components|Animation|PlayAnimation (Variables|Default|GetWeapon) "/Game/MilitaryWeapSilver/Weapons/Animations/Fire_Pistol_W.Fire_Pistol_W" false)
    (Variables|Default|SetCurrentBullets (- (Variables|Default|GetCurrentBullets) 1))))

(fn LineTrace
  (bind _returnvalue (Game|GetPlayerCharacter 0))
  (bind _distance_shoot (Variables|Default|GetDistance%20shoot))
  (bind _asplayer_character (Utilities|Casting|CastToPlayer_character _returnvalue))
  (bind _currentweapon (Variables|/Game/ThirdPerson/Blueprints/Player_character.Player_character_C|GetCurrentWeapon _asplayer_character))
  (bind _scene (Variables|/Game/Bluprints/weapon/BP_BaseWeapon.BP_BaseWeapon_C|GetScene _currentweapon))
  (bind _socket_name (Variables|/Game/Bluprints/weapon/BP_BaseWeapon.BP_BaseWeapon_C|GetSocket%20name _currentweapon))
  (bind _returnvalue_2 (Transformation|GetSocketLocation _scene _socket_name))
  (bind _returnvalue_3 (Transformation|GetSocketRotation _scene _socket_name))
  (bind _returnvalue_4 (Math|Vector|GetForwardVector _returnvalue_3))
  (bind _returnvalue_5 (* _returnvalue_4 _distance_shoot))
  (bind _returnvalue_6 (+ _returnvalue_2 _returnvalue_5))
  ;[1 1 1] Trace from Muzzle
  (bind (_outhit _returnvalue_7) (Collision|LineTraceByChannel _returnvalue_2 _returnvalue_6 "TraceTypeQuery2" false (Utilities|Array|MakeArray _asplayer_character 0) "None"))
  ;[1 1 1] Laser crosshair
  (if _returnvalue_7
    (bind _returnvalue_8 (Rendering|Decal|SpawnDecalatLocation "/Game/Bluprints/weapon/BulletMat/Laser_Mat_Inst.Laser_Mat_Inst" (Variables|Default|GetSizeOfLaser) (.ImpactPoint (Collision|BreakHitResult _outhit)) (Math|Rotator|FindLookatRotation _returnvalue_6 (.ImpactPoint (Collision|BreakHitResult _outhit))) 0.01))
    (Rendering|Components|Decal|SetFadeScreenSize _returnvalue_8 0.0001)
    (bind _asbp_guard (Utilities|Casting|CastToBP_Guard (.HitActor (Collision|BreakHitResult _outhit)))
      (:then
        (Game|Damage|ApplyDamage _asbp_guard (Variables|Default|GetDamage) 0 0))
      (:CastFailed
        _))
    (return "0, 0, 0" (.ImpactPoint (Collision|BreakHitResult _outhit)) (.HitActor (Collision|BreakHitResult _outhit)))))

(fn SpawnDecalTracer
  (params (Location :type Vector) (SpawnTransform :type Vector) (ImpactPoint :type Vector))
  (bind _returnvalue (Game|GetPlayerCharacter 0))
  (bind _scene (Variables|Default|GetScene))
  (bind _asplayer_character (Utilities|Casting|CastToPlayer_character _returnvalue))
  (bind _currentweapon (Variables|/Game/ThirdPerson/Blueprints/Player_character.Player_character_C|GetCurrentWeapon _asplayer_character))
  (bind _socket_name (Variables|/Game/Bluprints/weapon/BP_BaseWeapon.BP_BaseWeapon_C|GetSocket%20name _currentweapon))
  ;[1 1 1] Spawn bullet decal
  (Game|SpawnActorfromClass "/Game/Bluprints/weapon/BulletDecal/BulletDecal_BP.BulletDecal_BP_C" (Math|Transform|MakeTransform SpawnTransform (Math|Conversions|RotationFromXVector ImpactPoint) "0.025000,0.025000,0.025000") "AlwaysSpawn" 0 0)
  ;[1 1 1] Spawn Physic Bullet and tracer
  (if (>= (Math|Random|RandomIntegerinRange 1 10) 0)
    (Game|SpawnActorfromClass (Variables|Default|GetBulletClass) (Math|Transform|MakeTransform (Transformation|GetSocketLocation _scene _socket_name) (Math|Conversions|RotationFromXVector (Math|Vector|GetForwardVector (Transformation|GetSocketRotation _scene _socket_name)))) "AlwaysSpawn" 0 0))
  (return))

(fn LaserfromWeapon
  (bind _returnvalue (Game|GetPlayerCharacter 0))
  (bind _distance_shoot (Variables|Default|GetDistance%20shoot))
  (bind _asplayer_character (Utilities|Casting|CastToPlayer_character _returnvalue))
  (bind _currentweapon (Variables|/Game/ThirdPerson/Blueprints/Player_character.Player_character_C|GetCurrentWeapon _asplayer_character))
  (bind _scene (Variables|/Game/Bluprints/weapon/BP_BaseWeapon.BP_BaseWeapon_C|GetScene _currentweapon))
  (bind _socket_name (Variables|/Game/Bluprints/weapon/BP_BaseWeapon.BP_BaseWeapon_C|GetSocket%20name _currentweapon))
  (bind _returnvalue_2 (Transformation|GetSocketLocation _scene _socket_name))
  (bind _returnvalue_3 (Transformation|GetSocketRotation _scene _socket_name))
  (bind _returnvalue_4 (Math|Vector|GetForwardVector _returnvalue_3))
  (bind _returnvalue_5 (* _returnvalue_4 _distance_shoot))
  (bind _returnvalue_6 (+ _returnvalue_2 _returnvalue_5))
  ;[1 1 1] Trace from Muzzle
  (bind (_outhit _returnvalue_7) (Collision|LineTraceByChannel _returnvalue_2 _returnvalue_6 "TraceTypeQuery2" false (Utilities|Array|MakeArray _asplayer_character 0) "None"))
  ;[1 1 1] Laser crosshair
  (if _returnvalue_7
    (bind _returnvalue_8 (Rendering|Decal|SpawnDecalatLocation "/Game/Bluprints/weapon/BulletMat/Laser_Mat_Inst.Laser_Mat_Inst" (Variables|Default|GetSizeOfLaser) (.ImpactPoint (Collision|BreakHitResult _outhit)) (Math|Rotator|FindLookatRotation _returnvalue_6 (.ImpactPoint (Collision|BreakHitResult _outhit))) 0.015))
    (Rendering|Components|Decal|SetFadeScreenSize _returnvalue_8 0.0001)))