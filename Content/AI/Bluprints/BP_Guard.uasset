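; BP_Guard is an AI guard character that carries a weapon and exposes its team ID, death status and patrol route.
; BeginPlay spawns the weapon class and snaps it to the mesh's weapon socket.
; ChangeState forwards the new state to the animation instance, while ModifyMovementSpeed maps alert states to walk speeds.
; The health component's death event triggers a one-time ragdoll, disables capsule collision and prints a debug message.
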(event OnDamageTaken(Health_component))

(event OnDead(Health_component)
  (Utilities|FlowControl|DoOnce false
    (:Completed
      (Collision|SetCollisionProfileName (Variables|Character|GetMesh) "Ragdoll" true :!class /Script/Engine.PrimitiveComponent)
      (Class|SkeletalMeshComponent|SetAllBodiesSimulatePhysics (Variables|Character|GetMesh) true)
      (Collision|SetCollisionEnabled (Variables|Collision|GetCapsuleComponent) "NoCollision")
      (Development|PrintString (Utilities|String|Append (Utilities|GetDisplayName self) "Dead")))))

(event EventBeginPlay
  (bind _self self)
  (bind _returnvalue (Game|SpawnActorfromClass (Variables|Default|GetWeaponClass) (Math|Transform|MakeTransform "0, 0, 0") "AlwaysSpawn" _self _self))
  (bind _output_get (Variables|Default|SetWeapon _returnvalue))
  (Transformation|AttachComponentToComponent _output_get (Variables|Character|GetMesh) "WeaponSocket" "SnapToTarget" "SnapToTarget" "SnapToTarget" true))

(event Collision|EventActorBeginOverlap
  (params (OtherActor :type Actor%20Object%20Reference)))

(event EventTick
  (params (DeltaSeconds :type Float%20%28single-precision%29)))

(event EventChangeState
  (params (NewState :type NPC_State%20Enum :default "NewEnumerator0"))
  (Class|AIHelper|ChangeState(Message) (Components|SkeletalMesh|GetAnimInstance (Variables|Character|GetMesh)) NewState))

(event EventModifyMovementSpeed
  (params (State :type NPC_State%20Enum :default "NewEnumerator0"))
  (Variables|/Script/Engine.CharacterMovementComponent|SetMaxWalkSpeed (Variables|Character|GetCharacterMovement) (Utilities|Select :Index State :NewEnumerator0 1.6e+02 :NewEnumerator1 3e+02 :NewEnumerator2 4e+02 :NewEnumerator3 6e+02 :NewEnumerator4 0.0)))

(fn ConstructionScript)

(fn GetTeamId
  (return false))

(fn IsDeath
  (return (Default|IsDeath? (Variables|Default|GetHealth_component))))

(fn PatrolRoute
  (return (Variables|Default|GetPatrol%20Route)))