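; Zombie enemy character with melee attacks, health, hit reactions and a floating name/HP bar that turns toward the player camera.
; Attacks stop movement and play a weighted-random one- or two-hand montage, gated by DoOnce until AttackEnded restores speed.
; Externally triggered events toggle hand collision, whose overlaps deal random damage through per-hand DoOnce gates.
; Taking damage can interrupt attacks with a stagger, and zero HP triggers animated death and delayed destruction.
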(event OnComponentBeginOverlap(Right_hand)
  (params (OverlappedComponent :type Primitive%20Component%20Object%20Reference) (OtherActor :type Actor%20Object%20Reference) (OtherComp :type Primitive%20Component%20Object%20Reference) (OtherBodyIndex :type Integer) (bFromSweep :type Boolean) (SweepResult :type Hit%20Result%20Structure%20%28by%20ref%29))
  ;[1 1 1] Нанесення урона
  (if (!= OtherActor self)
    (Utilities|FlowControl|DoOnce false
      (:Completed
        (Game|Damage|ApplyDamage OtherActor (Math|Random|RandomFloatinRange 5.0 15.0) 0 0)))))

(event OnComponentBeginOverlap(Left_hand)
  (params (OverlappedComponent :type Primitive%20Component%20Object%20Reference) (OtherActor :type Actor%20Object%20Reference) (OtherComp :type Primitive%20Component%20Object%20Reference) (OtherBodyIndex :type Integer) (bFromSweep :type Boolean) (SweepResult :type Hit%20Result%20Structure%20%28by%20ref%29))
  ;[1 1 1] Нанесення урона
  (if (!= OtherActor self)
    (Utilities|FlowControl|DoOnce false
      (:Completed
        (Game|Damage|ApplyDamage OtherActor (Math|Random|RandomFloatinRange 5.0 15.0) 0 0)))))

(event Custom|Event%20attack
  ;[1 1 1] Логіка атака мобіка
  (if (not (Variables|Default|GetisDeath?))
    (Utilities|FlowControl|DoOnce false
      (:Completed
        ;;[1 1 1] При атаці макс скорость 0
        (Variables|/Script/Engine.CharacterMovementComponent|SetMaxWalkSpeed (Variables|Character|GetCharacterMovement) 0.0)
        (if (Math|Random|RandomBoolwithWeight 0.7)
          ;;[1 1 1] Удари мобіка
          (Animation|PlayAnimMontage "/Game/Enemy/animation/Zombie_Attack_one_hand_Montage.Zombie_Attack_one_hand_Montage" 1.5 "None")
          (else
            (Animation|PlayAnimMontage "/Game/Enemy/animation/Zombie_Attack_two_hands_Montage.Zombie_Attack_two_hands_Montage" 1.5 "None")))))))

(event Custom|Attack%20ended
  ;[1 1 1] Логіка атака мобіка
  (Variables|/Script/Engine.CharacterMovementComponent|SetMaxWalkSpeed (Variables|Character|GetCharacterMovement) 3e+02)
  (Utilities|FlowControl|DoOnce false) ; enters at Reset
)

(event Custom|Stop%20force%20attack
  (Animation|StopAnimMontage "/Game/Enemy/animation/Zombie_Attack_one_hand_Montage.Zombie_Attack_one_hand_Montage")
  (Animation|StopAnimMontage "/Game/Enemy/animation/Zombie_Attack_two_hands_Montage.Zombie_Attack_two_hands_Montage")
  (Collision|SetCollisionEnabled (Variables|Default|GetRight_hand) "NoCollision")
  (Collision|SetCollisionEnabled (Variables|Default|GetLeft_hand) "NoCollision"))

(event Custom|refresh%20attack%20right%20hand
  ;[1 1 1] Нанесення урона
  (Utilities|FlowControl|DoOnce false) ; enters at Reset
)

(event Custom|Enabled_one_hand_collision
  ;[1 1 1] Колізія при одиничному ударі руки
  (Collision|SetCollisionEnabled (Variables|Default|GetRight_hand) "QueryOnly"))

(event Custom|refresh%20attack%20left%20hand
  ;[1 1 1] Нанесення урона
  (Utilities|FlowControl|DoOnce false) ; enters at Reset
)

(event Custom|Disabled_one_hand_collision
  ;[1 1 1] Колізія при одиничному ударі руки
  (Collision|SetCollisionEnabled (Variables|Default|GetRight_hand) "NoCollision")
  (CallFunction|RefreshAttackRightHand))

(event Custom|Enabled_two_hand_collision
  ;[1 1 1] Колізія при удари обома руками
  (Utilities|FlowControl|Sequence
    (:then_0
      (Collision|SetCollisionEnabled (Variables|Default|GetLeft_hand) "QueryOnly"))
    (:then_1
      (Collision|SetCollisionEnabled (Variables|Default|GetRight_hand) "QueryOnly"))))

(event Custom|disabled_two_hand_collision
  ;[1 1 1] Колізія при удари обома руками
  (Utilities|FlowControl|Sequence
    (:then_0
      (Collision|SetCollisionEnabled (Variables|Default|GetLeft_hand) "NoCollision"))
    (:then_1
      (Collision|SetCollisionEnabled (Variables|Default|GetRight_hand) "NoCollision")
      (CallFunction|RefreshAttackRightHand)
      (CallFunction|RefreshAttackLeftHand))))

(event Custom|death
  ;[1 1 1] Смерть мобіка
  (Variables|Default|SetisDeath? true)
  (Default|DeathonAnimBP (.AsZompie%20Anim%20BP (Utilities|Casting|CastToZompie_animBP (Components|SkeletalMesh|GetAnimInstance (Variables|Character|GetMesh)))))
  (Animation|StopAnimMontage "/Game/Enemy/animation/Zombie_Attack_one_hand_Montage.Zombie_Attack_one_hand_Montage")
  (Animation|StopAnimMontage "/Game/Enemy/animation/Zombie_Attack_two_hands_Montage.Zombie_Attack_two_hands_Montage")
  (Collision|SetCollisionEnabled (Variables|Collision|GetCapsuleComponent) "NoCollision")
  (Audio|PlaySoundatLocation "/Game/Enemy/music_zombie/death_groan_001_11759_Cue.death_groan_001_11759_Cue" "0, 0, 0" "0, 0, 0" 1.0 1.0 0.0 0 0 0 0)
  (Utilities|FlowControl|Sequence
    (:then_0
      (Utilities|FlowControl|Delay 1e+01)
      (Actor|DestroyActor))))

(event Custom|hit%20direction
  (Variables|Default|SetEnemy%20rotation (CallFunction|RotationEnemy))
  (if (Math|Random|RandomBoolwithWeight 0.4)
    (CallFunction|StopForceAttack)
    (bind _returnvalue (Animation|PlayAnimMontage "/Game/Enemy/animation/Zombie_Reaction_Hit_Montage.Zombie_Reaction_Hit_Montage" 1.0 "None"))
    (Utilities|FlowControl|Delay (/ _returnvalue 4.0))
    (CallFunction|AttackEnded)))

(event EventBeginPlay
  (Variables|Default|SetAs%20HP%20Bar%20Wighet (.AsHP%20Bar%20Wighet (Utilities|Casting|CastToHP_Bar_Wighet (UserInterface|GetUserWidgetObject (Variables|Default|GetHP_Bar)))))
  ;[1 1 1] Фіксуємо швидкість персонажа
  (Variables|Default|SetStart%20max%20speed (Variables|/Script/Engine.CharacterMovementComponent|GetMaxWalkSpeed (Variables|Character|GetCharacterMovement))))

(event Collision|EventActorBeginOverlap
  (params (OtherActor :type Actor%20Object%20Reference)))

(event EventTick
  (params (DeltaSeconds :type Float%20%28single-precision%29))
  (Utilities|FlowControl|Sequence
    (:then_0
      ;[1 1 1] Передача хп у віджет
      (Progress|SetPercent (Variables|/Game/Enemy/HP_Bar_Wighet.HP_Bar_Wighet_C|GetHP_Bar (Variables|Default|GetAs%20HP%20Bar%20Wighet)) (Math|Float|NormalizetoRange (Variables|Default|GetCurrent_HP) 0.0 (Variables|Default|Getmax_HP)))
      ;[1 1 1] Передача ім'я мобіка
      (Rendering|Components|TextRender|SetText (Variables|/Game/Enemy/HP_Bar_Wighet.HP_Bar_Wighet_C|GetMob_name (Variables|Default|GetAs%20HP%20Bar%20Wighet)) (Variables|Default|GetMob_name)))
    (:then_1
      ;[1 1 1] Слідкування за камерою віджета
      (Transformation|SetWorldRotation (Variables|Default|GetHP_Bar) (Math|Rotator|FindLookatRotation (Transformation|GetWorldLocation (Variables|Default|GetHP_Bar)) (Transformation|GetWorldLocation (Variables|/Game/ThirdPerson/Blueprints/Player_character.Player_character_C|GetCamera (.AsPlayer%20Character (Utilities|Casting|CastToPlayer_character (Game|GetPlayerCharacter 0)))))) false false))))

(event Game|Damage|EventAnyDamage
  (params (Damage :type Float%20%28single-precision%29) (DamageType :type Damage%20Type%20Object%20Reference) (InstigatedBy :type Controller%20Object%20Reference) (DamageCauser :type Actor%20Object%20Reference))
  ;[1 1 1] do damage
  (Variables|Default|SetLast%20hit%20actor DamageCauser)
  (if (not (Variables|Default|GetisDeath?))
    (CallFunction|HitDirection)
    (bind _output_get (Variables|Default|SetCurrent_HP (Math|Float|SelectFloat 0.0 (- (Variables|Default|GetCurrent_HP) Damage) (>= Damage (Variables|Default|GetCurrent_HP)))))
    (Utilities|FlowControl|Sequence
      (:then_0
        (if (Math|Random|RandomBoolwithWeight 1.0)
          (Audio|PlaySoundatLocation "/Game/Sound/Damage_and_death/damage_zombie_Cue.damage_zombie_Cue" "0, 0, 0" "0, 0, 0" 1.0 1.0 0.0 0 0 0 0)))
      (:then_1
        (if (<= _output_get 0.0)
          (CallFunction|Death)
          (Development|PrintString "Мобік вмер("))))))

(fn ConstructionScript)

(fn RotationEnemy
  (return (.Yaw (Math|Rotator|BreakRotator (Math|Rotator|Delta(Rotator) (Math|Rotator|FindLookatRotation (Transformation|GetActorLocation) (Transformation|GetActorLocation (Game|GetPlayerCharacter 0))) (Transformation|GetActorRotation))))))