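; AI controller for the zombie enemy that chases and attacks the player, or patrols around its spawn point.
; Each Tick, a macro uses a delayed distance check and the player's death state, without perception or line of sight, to choose the behavior.
; DoOnce gates throttle AIMoveTo: reaching a living player triggers the attack, otherwise the zombie wanders to random navmesh points.
; Movement stops once the zombie dies.
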(event EventBeginPlay
  (Utilities|FlowControl|Delay 0.2)
  (Variables|Default|SetAs%20Zombie%20BP (.AsZombie%20BP (Utilities|Casting|CastToZombie_BP (Pawn|GetControlledPawn))))
  ;[1 1 1] Місце спавну мобіка
  (Variables|Default|SetSpawn_location (Transformation|GetActorLocation (.AsZombie%20BP (Utilities|Casting|CastToZombie_BP (Pawn|GetControlledPawn)))))
  (Variables|Default|SetPause%20to%20start true))

(event EventTick
  (params (DeltaSeconds :type Float%20%28single-precision%29))
  (if (Variables|Default|GetPause%20to%20start)
    (if (not (Variables|/Game/Enemy/Zombie_BP.Zombie_BP_C|GetisDeath? (Variables|Default|GetAs%20Zombie%20BP)))
      (Utilities|AILookingforEnemy 1.6e+03
        (:see%20enemy
          ;[1 1 1] Атака мобіка по персонажа
          (Utilities|FlowControl|DoOnce false :!label _label
            (:Completed
              (AI|AIMoveTo (Variables|Default|GetAs%20Zombie%20BP) "0, 0, 0" (Game|GetPlayerCharacter 0) 85.0 false
                (:OnSuccess
                  (Default|EventAttack (Variables|Default|GetAs%20Zombie%20BP))
                  (goto _label Reset))
                (:OnFail
                  (goto _label Reset))))))
        (:see%20dead%20enemy
          _)
        (:dont%20see%20enemy
          _))
      ;[1 1 1] Патрулювання території
      (Utilities|FlowControl|DoOnce false :!label _label_2
        (:Completed
          (AI|AIMoveTo (Variables|Default|GetAs%20Zombie%20BP) (.RandomLocation (Class|NavigationSystemV1|GetRandomPointinNavigableRadius (Variables|Default|GetSpawn_location) 1.6e+03 0 0)) 0 5.0 false
            (:then
              _)
            (:OnSuccess
              _)
            (:OnFail
              _))
          (Utilities|FlowControl|Delay 5.0)
          (goto _label_2 Reset)))
      (else
        (Utilities|FlowControl|DoOnce false
          (:Completed
            (AI|Navigation|StopMovement)))))))

(fn ConstructionScript)